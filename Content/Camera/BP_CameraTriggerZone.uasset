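; A trigger zone that switches the third-person character to a fixed camera style while it overlaps the zone.
; On entry it attaches the character's gameplay camera rig parameter to FixedCameraActor, then saves any non-fixed camera style and sets the style tag to Camera.Style.Fixed.
; On exit it restores the style from that saved variable, leaving the rig attachment parameter unchanged.
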(event `self.ReceiveActorBeginOverlap`
  (params (OtherActor :type "Actor Object Reference"))
  (bind _asbp_third_person_character (cast `/Game/ThirdPerson/Blueprints/BP_ThirdPersonCharacter` OtherActor))
  (`|SetCameraRigParameter` (`GameplayCameraComponentBase.GetInitialResult` (`/Game/ThirdPerson/Blueprints/BP_ThirdPersonCharacter.GameplayCamera` _asbp_third_person_character)) (make `CameraActorAttachmentInfo` (`self.FixedCameraActor`)))
  (bind _camerastyle_ (`/Game/ThirdPerson/Blueprints/BP_ThirdPersonCharacter.CameraStyle ` _asbp_third_person_character))
  (if (not (`BlueprintGameplayTagLibrary.MatchesTag` _camerastyle_ (struct :`TagName` "Camera.Style.Fixed")))
    (set `self.TmpCameraStyle` _camerastyle_)
    (set `/Game/ThirdPerson/Blueprints/BP_ThirdPersonCharacter.CameraStyle ` (struct :`TagName` "Camera.Style.Fixed") _asbp_third_person_character)))

(event `self.ReceiveActorEndOverlap`
  (params (OtherActor :type "Actor Object Reference"))
  (bind _asbp_third_person_character (cast `/Game/ThirdPerson/Blueprints/BP_ThirdPersonCharacter` OtherActor))
  (set `/Game/ThirdPerson/Blueprints/BP_ThirdPersonCharacter.CameraStyle ` (`self.TmpCameraStyle`) _asbp_third_person_character))

(fn `UserConstructionScript`)