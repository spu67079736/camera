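; Lock-on component for BP_ThirdPersonCharacter that finds a nearby target and feeds it to the gameplay camera.
; SetFindTarget toggles a looping timer for the periodic search, clearing the lock when switched off.
; Despite its name, FindClosestTarget sphere-traces pawns around the player and takes the first lockable hit, without comparing distances.
; Each search writes the lock flag and camera-to-target vector into camera rig parameters.
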(event `self.ReceiveBeginPlay`
  (bind _asbp_third_person_character (cast `/Game/ThirdPerson/Blueprints/BP_ThirdPersonCharacter` (`self.GetOwner`)))
  (set `self.OwnerPlayer` _asbp_third_person_character)
  (set `self.IsFinding ` false))

(event `FindTarget_Event`
  (bind _gameplaycamera (`/Game/ThirdPerson/Blueprints/BP_ThirdPersonCharacter.GameplayCamera` (`self.OwnerPlayer`)))
  (bind _returnvalue (`GameplayCameraComponentBase.GetInitialResult` (`/Game/ThirdPerson/Blueprints/BP_ThirdPersonCharacter.GameplayCamera` (`self.OwnerPlayer`))))
  (bind _returnvalue_2 (`GameplayCameraComponentBase.GetInitialResult` _gameplaycamera))
  (if (`self.IsFinding `)
    (bind _output_get (set `self.LockTarget` (`self.FindClosestTarget`)))
    (if (`KismetSystemLibrary.IsValid` _output_get)
      (`|SetCameraRigParameter` _returnvalue_2 (- (`Actor.K2_GetActorLocation` (`self.LockTarget`)) (`SceneComponent.K2_GetComponentLocation` _gameplaycamera)))
      (`|SetCameraRigParameter` _returnvalue_2 true)
      (else
        (`|SetCameraRigParameter` _returnvalue)
        (`|SetCameraRigParameter` _returnvalue)))))

(fn `BPC_TargetLockComponent_AutoGenFunc`)

(fn `FindClosestTarget`
  (returns (NewParam :type "Actor Object Reference"))
  (locals (`ClosestTarget ` :type "Actor Object Reference"))
  (bind _returnvalue (`Actor.K2_GetActorLocation` (`self.OwnerPlayer`)))
  (bind (_outhits _returnvalue_2) (`KismetSystemLibrary.SphereTraceMultiForObjects` _returnvalue _returnvalue 300.0 (`|MakeArray` "ObjectTypeQuery3" :!type "EObjectTypeQuery Enum")))
  (if _returnvalue_2
    (for _array_element _outhits
      (bind (_bblockinghit _binitialoverlap _time _distance _location _impactpoint _normal _impactnormal _physmat _hitactor) (`GameplayStatics.BreakHitResult` _array_element))
      (bind _newparam (message `/Game/Camera/BPI_TargetLockable.IsTargetLockable` _hitactor))
      (if _newparam
        (set `local.ClosestTarget ` _hitactor)
        (break))))
  (return (`local.ClosestTarget `)))

(fn `GetFindingTarget`
  (returns (NewParam :type Boolean))
  (return (`self.IsFinding `)))

(fn `SetFindTarget`
  (params (NewParam :type Boolean))
  (bind _returnvalue (`GameplayCameraComponentBase.GetInitialResult` (`/Game/ThirdPerson/Blueprints/BP_ThirdPersonCharacter.GameplayCamera` (`self.OwnerPlayer`))))
  (bind _output_get (set `self.IsFinding ` NewParam))
  (if _output_get
    (bind _returnvalue_2 (`KismetSystemLibrary.K2_SetTimerDelegate` (`|CreateDelegate` :!event `FindTarget_Event`) 0.2 true))
    (set `self.FindTargetTimer` _returnvalue_2)
    (else
      (`KismetSystemLibrary.K2_ClearAndInvalidateTimerHandle` (`self.FindTargetTimer`))
      (set `self.LockTarget` null)
      (`|SetCameraRigParameter` _returnvalue)
      (`|SetCameraRigParameter` _returnvalue))))